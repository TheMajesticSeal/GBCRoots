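; BP_Root is an actor that trails a chain of mesh instances behind it, forming a root-like body that follows its movement.
; The construction script detaches the RootBody instanced mesh and lays out RootLength-driven instances in a line along negative X.
; While moving, Tick snapshots all instance transforms, snaps the first to the actor, then eases each later one toward its predecessor's snapshot for a lagging follow effect.
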(event `self.ReceiveTick`
  (params (DeltaSeconds :type "Float (single-precision)"))
  (if (> (`KismetMathLibrary.VSize` (`self.GetVelocity`)) 10.0)
    (`self.LerpLocations`)))

(event `LerpLocations`
  (bind (_returnvalue_location _returnvalue_rotation) (`KismetMathLibrary.BreakTransform` (`self.GetTransform`)))
  (bind _rootbody (`self.RootBody`))
  (bind (_output_location _output_rotation _output_scale) (`KismetMathLibrary.BreakTransform` (`|GetArrayItem` (`self.InstanceTransorms`))))
  (`KismetArrayLibrary.Array_Clear` (`self.InstanceTransorms`))
  (for _index (range (+ (- (`InstancedStaticMeshComponent.GetInstanceCount` (`self.RootBody`)) 0) 1))
    (`KismetArrayLibrary.Array_Add` (`self.InstanceTransorms`) (`InstancedStaticMeshComponent.GetInstanceTransform` (`self.RootBody`) _index true)))
  (`InstancedStaticMeshComponent.UpdateInstanceTransform` (`self.RootBody`) 0 (`KismetMathLibrary.MakeTransform` _returnvalue_location _returnvalue_rotation _output_scale) true true false)
  (for (_array_element _array_index) (`self.InstanceTransorms`)
    (bind _returnvalue (+ _array_index 1))
    (`InstancedStaticMeshComponent.UpdateInstanceTransform` _rootbody _returnvalue (`KismetMathLibrary.TLerp` (`InstancedStaticMeshComponent.GetInstanceTransform` _rootbody _returnvalue true) _array_element 0.05) true true false)))

(fn `UserConstructionScript`
  (bind _rootbody (`self.RootBody`))
  (`parent.UserConstructionScript`)
  (`SceneComponent.K2_DetachFromComponent` _rootbody "KeepWorld" "KeepWorld" "KeepWorld" true)
  (`InstancedStaticMeshComponent.ClearInstances` _rootbody)
  (for _index (range (+ (`self.RootLength`) 1))
    (`InstancedStaticMeshComponent.AddInstance` (`self.RootBody`) (`KismetMathLibrary.MakeTransform` (`KismetMathLibrary.MakeVector` (`KismetMathLibrary.Conv_IntToDouble` (* _index -60))) (struct) (0.5 0.5 0.5)) false)))