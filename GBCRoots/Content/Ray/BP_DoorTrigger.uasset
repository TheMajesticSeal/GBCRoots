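; BP_DoorTrigger is a box trigger that opens the matching BP_Door when a BP_Root actor enters it.
; On overlap it searches all BP_Door actors, opening any whose ID equals its own and calling ShowMSG on every other door.
; It remembers the last opened door and closes it when the BP_Root actor leaves the box.
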(event `self.Box.OnComponentBeginOverlap`
  (params (OverlappedComponent :type "PrimitiveComponent Object Reference") (OtherActor :type "Actor Object Reference") (OtherComp :type "PrimitiveComponent Object Reference") (OtherBodyIndex :type Integer) (bFromSweep :type Boolean) (SweepResult :type "HitResult Structure (by ref)"))
  (cast `/Game/Ray/BP_Root` OtherActor)
  (bind _outactors (`GameplayStatics.GetAllActorsOfClass` "/Game/Ray/BP_Door.BP_Door_C"))
  (for _array_element _outactors
    (if (== (`/Game/Ray/BP_Door.ID` _array_element) (`self.ID`))
      (`/Game/Ray/BP_Door.OpenDoor` _array_element)
      (set `self.LastOpenedDoor` _array_element)
      (else
        (`/Game/Ray/BP_Door.ShowMSG` _array_element)))))

(event `self.Box.OnComponentEndOverlap`
  (params (OverlappedComponent :type "PrimitiveComponent Object Reference") (OtherActor :type "Actor Object Reference") (OtherComp :type "PrimitiveComponent Object Reference") (OtherBodyIndex :type Integer))
  (bind _lastopeneddoor (`self.LastOpenedDoor`))
  (cast `/Game/Ray/BP_Root` OtherActor)
  (`/Engine/EditorBlueprintResources/StandardMacros.IsValid` _lastopeneddoor
    (:`Is Valid`
      (`/Game/Ray/BP_Door.CloseDoor` _lastopeneddoor))))

(fn `UserConstructionScript`)